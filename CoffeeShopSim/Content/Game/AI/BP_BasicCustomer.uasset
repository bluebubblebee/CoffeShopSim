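; BP_BasicCustomer is an AI shop customer character driven by the BT_Customer behavior tree.
; On BeginPlay it caches its anim instance, starts the tree and seeds the blackboard with the player and its start location.
; Events for counter, waiting area, exit and order completion write blackboard targets and a CustomerStatus enum that the tree reads.
; A stand-up event briefly pulses an animation flag.
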(event `OnStandingUp`
  (bind _bpa_animator (`self.BPA_Animator`))
  (if (`KismetSystemLibrary.IsValid` _bpa_animator)
    (set `/Game/Game/Art/Characters/BPA_BasicCharacter.IsStandingUp` true _bpa_animator)
    (`KismetSystemLibrary.Delay` 0.2)
    (set `/Game/Game/Art/Characters/BPA_BasicCharacter.IsStandingUp` false _bpa_animator)))

(event `self.ReceiveBeginPlay`
  (bind _asbpa_basic_character (cast `/Game/Game/Art/Characters/BPA_BasicCharacter` (`SkeletalMeshComponent.GetAnimInstance` (`self.Mesh`))))
  (set `self.BPA_Animator` _asbpa_basic_character)
  (`AIController.RunBehaviorTree` (`AIBlueprintHelperLibrary.GetAIController` self) "/Game/Game/AI/BT_Customer.BT_Customer")
  (`self.InitializeBlackboard`))

(event `self.OnGotoCounter`
  (params (CounterLocation :type "Actor Object Reference") (ObjectToLookAt :type "Actor Object Reference"))
  (bind _returnvalue (`AIBlueprintHelperLibrary.GetBlackboard` (`AIBlueprintHelperLibrary.GetAIController` self)))
  (`BlackboardComponent.SetValueAsObject` _returnvalue "CounterShopActor" CounterLocation)
  (`BlackboardComponent.SetValueAsObject` _returnvalue "ObjectToLookAt" ObjectToLookAt)
  (`self.UpdateCustomerStatus` "VE_GoToCounter"))

(event `self.OnGotoWaitLocation`
  (params (WaitLocation :type "Vector Structure") (ObjectToLookAt :type "Actor Object Reference"))
  (bind _returnvalue (`AIBlueprintHelperLibrary.GetBlackboard` (`AIBlueprintHelperLibrary.GetAIController` self)))
  (`BlackboardComponent.SetValueAsVector` _returnvalue "WaitingLocation" WaitLocation)
  (`BlackboardComponent.SetValueAsObject` _returnvalue "ObjectToLookAt" ObjectToLookAt)
  (`self.UpdateCustomerStatus` "VE_GoToWaitingArea"))

(event `self.OnExitShop`
  (`self.UpdateCustomerStatus` "VE_ExitShop"))

(event `self.OnOrderCompleted`
  (`self.UpdateCustomerStatus` "VE_ExitShop"))

(fn `InitializeBlackboard`
  (bind _returnvalue (`AIBlueprintHelperLibrary.GetBlackboard` (`AIBlueprintHelperLibrary.GetAIController` self)))
  (`BlackboardComponent.SetValueAsObject` _returnvalue "Player" (`GameplayStatics.GetPlayerCharacter` 0))
  (`BlackboardComponent.SetValueAsVector` _returnvalue "StartLocation" (`self.K2_GetActorLocation`)))

(fn `UpdateCustomerStatus`
  (params (Status :type "ECustomerStatus Enum" :default "VE_None"))
  (bind _output_get (set `self.CustomerStatus` Status))
  (`BlackboardComponent.SetValueAsEnum` (`AIBlueprintHelperLibrary.GetBlackboard` (`AIBlueprintHelperLibrary.GetAIController` self)) "CustomerStatus" _output_get))

(fn `UserConstructionScript`)
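; Coffee shop manager that moves pooled customers in and out of the shop when its interactive door opens or closes.
; On door open, the first customer goes to the counter, then a self-calling event sends others to random points around the waiting area at random intervals until the shop limit is reached.
; On door close, a delayed loop sends customers out in reverse order, counting down the in-shop total.
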(event `self.ReceiveBeginPlay`
  (bind _doorinteractive (`self.DoorInteractive`))
  (`/Engine/EditorBlueprintResources/StandardMacros.IsValid` _doorinteractive
    (:`Is Valid`
      (add `DoorInteractive.OnDoorOpened` _doorinteractive (delegate `OnShopDoorOpened`))
      (add `DoorInteractive.OnDoorClosed` _doorinteractive (delegate `OnShopDoorClosed`)))))

(event `OnShopDoorOpened`
  (`self.OnDoorOpened`))

(event `OnShopDoorClosed`
  (`self.OnDoorClosed`))

(event `OnDoorOpened`
  (`NPCCustomer.OnGotoCounter` (`|GetArrayItem` (`self.CustomerPoolList`)) (`self.CounterLocation`) (`self.ObjectToLookAt`))
  (`self.OnSendNewCustomer`))

(event `OnSendNewCustomer`
  (`KismetSystemLibrary.Delay` (`KismetMathLibrary.RandomFloatInRange` 2.0 4.0))
  (bind _output_get (set `self.CustomersInShop` (+ (`self.CustomersInShop`) 1)))
  (`NPCCustomer.OnGotoWaitLocation` (`|GetArrayItem` (`self.CustomerPoolList`) _output_get) (`KismetMathLibrary.RandomPointInBoundingBox` (`self.K2_GetActorLocation` (`self.WaitingAreaLocation`)) (500.0 500.0 0.0)) (`self.ObjectToLookAt`))
  (if (< (`self.CustomersInShop`) (`self.MaxCustomerInShop`))
    (`self.OnSendNewCustomer`)))

(event `OnDoorClosed`
  (`NPCCustomer.OnExitShop` (`|GetArrayItem` (`self.CustomerPoolList`) (`self.CustomersInShop`)) :!label _label)
  (bind _output_get (set `self.CustomersInShop` (- (`self.CustomersInShop`) 1)))
  (if (>= _output_get 0)
    (`KismetSystemLibrary.Delay` 2.0)
    (goto _label)))

(fn `UserConstructionScript`)
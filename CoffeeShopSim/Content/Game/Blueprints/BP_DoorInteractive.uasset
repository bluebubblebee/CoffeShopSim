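; BP_DoorInteractive is an interactive double door that registers with CoffeeShopSimCharacter while the player overlaps its trigger.
; OnInteract opens it by hiding both door meshes, then setting IsOpen and firing the opened dispatcher after delays.
; Closing fires the closed dispatcher immediately and shows the meshes after a delay.
; LockInteractive blocks re-entry; opening releases it after a delay, while closing never clears it here.
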(event `self.Trigger.OnComponentBeginOverlap`
  (params (OverlappedComponent :type "PrimitiveComponent Object Reference") (OtherActor :type "Actor Object Reference") (OtherComp :type "PrimitiveComponent Object Reference") (OtherBodyIndex :type Integer) (bFromSweep :type Boolean) (SweepResult :type "HitResult Structure (by ref)"))
  (bind _ascoffee_shop_sim_character (cast `CoffeeShopSimCharacter` OtherActor))
  (`CoffeeShopSimCharacter.OnEnterInteractive` _ascoffee_shop_sim_character self (`self.InteractiveName`)))

(event `self.Trigger.OnComponentEndOverlap`
  (params (OverlappedComponent :type "PrimitiveComponent Object Reference") (OtherActor :type "Actor Object Reference") (OtherComp :type "PrimitiveComponent Object Reference") (OtherBodyIndex :type Integer))
  (bind _ascoffee_shop_sim_character (cast `CoffeeShopSimCharacter` OtherActor))
  (`CoffeeShopSimCharacter.OnLeaveInteractive` _ascoffee_shop_sim_character))

(event `self.OnInteract`
  (if (`self.LockInteractive`)
    _
    (elif (`self.bIsOpen`)
      (`|ExecutionSequence`
        (:`then_0`
          (set `self.LockInteractive` true))
        (:`then_1`
          (`self.OnDoorClosed`))
        (:`then_2`
          (`KismetSystemLibrary.Delay` 10.0)
          (`|ExecutionSequence`
            (:`then_0`
              (`SceneComponent.SetVisibility` (`self.LeftDoor`) true false))
            (:`then_1`
              (`SceneComponent.SetVisibility` (`self.RightDoor`) true false))))
        (:`then_3`
          (set `self.bIsOpen` false)))
      (else
        (`|ExecutionSequence`
          (:`then_0`
            (set `self.LockInteractive` true))
          (:`then_1`
            (`SceneComponent.SetVisibility` (`self.LeftDoor`) false false))
          (:`then_2`
            (`SceneComponent.SetVisibility` (`self.RightDoor`) false false))
          (:`then_3`
            (`KismetSystemLibrary.Delay` 2.0)
            (set `self.bIsOpen` true)
            (`self.OnDoorOpened`)
            (`KismetSystemLibrary.Delay` 5.0)
            (set `self.LockInteractive` false)))))))

(fn `UserConstructionScript`)
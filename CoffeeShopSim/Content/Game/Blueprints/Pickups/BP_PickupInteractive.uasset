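; Base interactive pickup for the coffee shop sim that lets the player character know when it is in range to interact.
; On trigger overlap it caches the CoffeeShopSimCharacter, passes it itself and its InteractiveName, then calls OnPlayerEnterInteractive.
; When that same character leaves, it notifies the character, clears the reference and calls OnPlayerLeaveInteractive.
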(event `self.Trigger.OnComponentBeginOverlap`
  (params (OverlappedComponent :type "PrimitiveComponent Object Reference") (OtherActor :type "Actor Object Reference") (OtherComp :type "PrimitiveComponent Object Reference") (OtherBodyIndex :type Integer) (bFromSweep :type Boolean) (SweepResult :type "HitResult Structure (by ref)"))
  ;[0.7765 0.4549 1] Trigger Interaction
  (bind _ascoffee_shop_sim_character (cast `CoffeeShopSimCharacter` OtherActor))
  (set `self.PlayerCharacter` _ascoffee_shop_sim_character)
  (`CoffeeShopSimCharacter.OnEnterInteractive` _ascoffee_shop_sim_character self (`self.InteractiveName`))
  (`self.OnPlayerEnterInteractive`))

(event `self.Trigger.OnComponentEndOverlap`
  (params (OverlappedComponent :type "PrimitiveComponent Object Reference") (OtherActor :type "Actor Object Reference") (OtherComp :type "PrimitiveComponent Object Reference") (OtherBodyIndex :type Integer))
  (bind _playercharacter (`self.PlayerCharacter`))
  ;[0.7765 0.4549 1] Trigger Interaction
  (bind _ascoffee_shop_sim_character (cast `CoffeeShopSimCharacter` OtherActor))
  (if (== _ascoffee_shop_sim_character _playercharacter)
    (`CoffeeShopSimCharacter.OnLeaveInteractive` _playercharacter)
    (set `self.PlayerCharacter` null)
    (`self.OnPlayerLeaveInteractive`)))

(fn `UserConstructionScript`)
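; Player Blueprint for an order-serving game, linking interaction, item handling and customer order events to the player HUD.
; It creates WBP_PlayerUI on BeginPlay, then forwards interactable names, orders, completed items and, after a short delay, coin updates.
; It extends parent item events by spawning the received item's actor attached to ItemSpawner as the held item, and destroying it when given away.
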(event `self.ReceiveBeginPlay`
  (bind _returnvalue (`|CreateWidget` "/Game/Game/ui/WBP_PlayerUI.WBP_PlayerUI_C"))
  (`UserWidget.AddToViewport` _returnvalue 0)
  (set `self.UI` _returnvalue))

(event `OnCustomerOrder`
  (params (Customer :type "Customer Structure") (Order :type "Order Structure"))
  (bind _ui (`self.UI`))
  (bind _output_get (set `self.CurrentCustomer` Customer))
  (bind _output_get_2 (set `self.CurrentOrder` Order))
  (`/Engine/EditorBlueprintResources/StandardMacros.IsValid` _ui
    (:`Is Valid`
      (`/Game/Game/ui/WBP_PlayerUI.OnShowOrder` _ui _output_get _output_get_2))))

(event `self.OnEnterInteractive`
  (params (InteractiveActor :type "Actor Object Reference") (InteractiveName :type Name))
  (`parent.OnEnterInteractive` InteractiveActor InteractiveName)
  (`/Game/Game/ui/WBP_PlayerUI.ShowTitle` (`self.UI`) (`KismetTextLibrary.Conv_NameToText` InteractiveName)))

(event `self.OnLeaveInteractive`
  (bind _ui (`self.UI`))
  (`parent.OnLeaveInteractive`)
  (`/Engine/EditorBlueprintResources/StandardMacros.IsValid` _ui
    (:`Is Valid`
      (`/Game/Game/ui/WBP_PlayerUI.HideTitle` _ui))))

(event `self.OnReceiveItem`
  (params (Item :type "Item Structure"))
  (bind _itemspawner (`self.ItemSpawner`))
  (`parent.OnReceiveItem` Item)
  (bind _returnvalue (`|SpawnActorFromClass` (`.ItemClass` (break `Item` Item)) (`KismetMathLibrary.MakeTransform` (`SceneComponent.K2_GetComponentLocation` _itemspawner) (`SceneComponent.K2_GetComponentRotation` _itemspawner)) "Undefined" "SelectDefaultAtRuntime" null null))
  (`self.K2_AttachToComponent` _returnvalue (`self.ItemSpawner`) "Fist_LSocket" "KeepWorld" "KeepWorld" "KeepWorld" true)
  (set `self.ItemOnHands_0` _returnvalue))

(event `self.OnGiveItem`
  (`parent.OnGiveItem`)
  (`self.K2_DestroyActor` (`self.ItemOnHands_0`)))

(event `self.OnOrderItemCompleted`
  (params (ItemID :type Name))
  (`/Game/Game/ui/WBP_PlayerUI.OnCompleteItemOrder` (`self.UI`) ItemID))

(event `self.OnOrderCompleted`
  (params (Coins :type Integer))
  (bind _ui (`self.UI`))
  (`KismetSystemLibrary.Delay` 2.0)
  (`/Game/Game/ui/WBP_PlayerUI.OnUpdateCoins` _ui Coins)
  (`/Game/Game/ui/WBP_PlayerUI.OnHideOrder` _ui))

(fn `UserConstructionScript`)
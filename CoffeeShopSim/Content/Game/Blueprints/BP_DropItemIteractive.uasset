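; Drop-off interactive in the coffee shop sim where the player places items to fulfil the current order.
; A trigger registers and unregisters the actor with the player character on overlap.
; Each drop locks the interactive, spawns the item at one of three slots by item count, and asks the game mode's ShopManager whether the order is complete.
; Completion clears the items and spawned actors; either outcome unlocks after a short delay.
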(event `self.Trigger.OnComponentBeginOverlap`
  (params (OverlappedComponent :type "PrimitiveComponent Object Reference") (OtherActor :type "Actor Object Reference") (OtherComp :type "PrimitiveComponent Object Reference") (OtherBodyIndex :type Integer) (bFromSweep :type Boolean) (SweepResult :type "HitResult Structure (by ref)"))
  ;[0.7765 0.4549 1] Trigger Interaction
  (bind _ascoffee_shop_sim_character (cast `CoffeeShopSimCharacter` OtherActor))
  (set `self.PlayerCharacter` _ascoffee_shop_sim_character)
  (`CoffeeShopSimCharacter.OnEnterInteractive` _ascoffee_shop_sim_character self (`self.InteractiveName`))
  (`self.OnPlayerEnterInteractive`))

(event `self.Trigger.OnComponentEndOverlap`
  (params (OverlappedComponent :type "PrimitiveComponent Object Reference") (OtherActor :type "Actor Object Reference") (OtherComp :type "PrimitiveComponent Object Reference") (OtherBodyIndex :type Integer))
  (bind _playercharacter (`self.PlayerCharacter`))
  ;[0.7765 0.4549 1] Trigger Interaction
  (bind _ascoffee_shop_sim_character (cast `CoffeeShopSimCharacter` OtherActor))
  (if (== _ascoffee_shop_sim_character _playercharacter)
    (`CoffeeShopSimCharacter.OnLeaveInteractive` _playercharacter)
    (set `self.PlayerCharacter` null)
    (`self.OnPlayerLeaveInteractive`)))

(event `self.OnItemDropped`
  (params (Item :type "Item Structure (by ref)"))
  (bind (_itemid _name _itemclass) (break `Item` Item))
  (set `self.LockInteractive` true)
  (`self.Spawn Item Mesh` _itemclass)
  (bind _ascoffee_shop_sim_game_mode (cast `CoffeeShopSimGameMode` (`GameplayStatics.GetGameMode`)))
  (bind _returnvalue (`ShopManager.CheckIfCurrentOrderCompleted` (`CoffeeShopSimGameMode.ShopManager` _ascoffee_shop_sim_game_mode) _itemid))
  (if _returnvalue
    (`KismetArrayLibrary.Array_Clear` (`self.ItemsOnInteractive`))
    (bind (_arrayindex _arrayelement) (`/Engine/EditorBlueprintResources/StandardMacros.ReverseForEachLoop` (`self.MeshItemList`))
      (:`LoopBody`
        (if (`KismetSystemLibrary.IsValid` _arrayelement)
          (`self.K2_DestroyActor` _arrayelement)))
      (:`Completed`
        (`KismetArrayLibrary.Array_Clear` (`self.MeshItemList`))
        (`KismetSystemLibrary.Delay` 1.0)
        (set `self.LockInteractive` false)))
    (else
      (`KismetSystemLibrary.Delay` 0.5)
      (set `self.LockInteractive` false))))

(fn `Spawn Item Mesh`
  (params (ItemMesh :type "Actor Class Reference"))
  (switch `int` (- (`KismetArrayLibrary.Array_Length` (`self.ItemsOnInteractive`)) 1)
    (:`0`
      (bind _returnvalue (`|SpawnActorFromClass` ItemMesh (`KismetMathLibrary.MakeTransform` (`SceneComponent.K2_GetComponentLocation` (`self.ItemDrop0`))) "AlwaysSpawn" "SelectDefaultAtRuntime" null null))
      (`KismetArrayLibrary.Array_Add` (`self.MeshItemList`) _returnvalue))
    (:`1`
      (bind _returnvalue_2 (`|SpawnActorFromClass` ItemMesh (`KismetMathLibrary.MakeTransform` (`SceneComponent.K2_GetComponentLocation` (`self.ItemDrop1`))) "AlwaysSpawn" "SelectDefaultAtRuntime" null null))
      (`KismetArrayLibrary.Array_Add` (`self.MeshItemList`) _returnvalue_2))
    (:`2`
      (bind _returnvalue_3 (`|SpawnActorFromClass` ItemMesh (`KismetMathLibrary.MakeTransform` (`SceneComponent.K2_GetComponentLocation` (`self.ItemDrop2`))) "AlwaysSpawn" "SelectDefaultAtRuntime" null null))
      (`KismetArrayLibrary.Array_Add` (`self.MeshItemList`) _returnvalue_3))))

(fn `UserConstructionScript`)
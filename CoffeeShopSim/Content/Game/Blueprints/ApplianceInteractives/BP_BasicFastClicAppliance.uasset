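; Base coffee-shop appliance that runs a fast-click minigame to give the player a recipe.
; A trigger registers it with the character, and each interact advances a state machine: select recipe, count clicks, then deliver.
; Starting locks and snaps the player to a marked position and shows a progress widget driven by click count.
; An interact after the bar fills attempts delivery, unlocks the player and, on success, plays a mesh scale timeline.
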(event `self.ReceiveBeginPlay`
  (bind _widget (`self.Widget`))
  ;[0 0.7654 1] Begin Play
  (`SceneComponent.SetVisibility` _widget false false)
  (bind _aswbp_fast_click (cast `/Game/Game/ui/WBP_FastClick` (`WidgetComponent.GetWidget` _widget)))
  (set `self.WBPFastClick` _aswbp_fast_click))

(event `self.OnPlayerEnterInteractive`
  ;[0.385 0.8006 1] Player Enter/Leaves Trigger
  (set `self.State` 0)
  (set `self.CurrentNumberClicks` 0))

(event `self.OnInteract`
  ;[0.08206 0.7201 1] Interact
  (`parent.OnInteract`)
  (switch `int` (`self.State`)
    (:`0`
      (bind _returnvalue (`self.TryToSelectRecipe`))
      (if _returnvalue
        (`self.LockPlayer`)
        (`self.OnStartMinigame`)))
    (:`1`
      (`self.OnUpdateMinigame`))
    (:`2`
      (`self.OnCompleteMinigame`))))

(event `self.OnPlayerLeaveInteractive`
  ;[0.385 0.8006 1] Player Enter/Leaves Trigger
  (set `self.State` 0)
  (set `self.CurrentNumberClicks` 0))

(event `self.OnStartMinigame`
  (bind _wbpfastclick (`self.WBPFastClick`))
  (set `self.CurrentNumberClicks` 0)
  (`SceneComponent.SetVisibility` (`self.Widget`) true false)
  (`/Game/Game/ui/WBP_FastClick.SetProgress` _wbpfastclick 0.0)
  (`/Game/Game/ui/WBP_FastClick.PlayPressLoop` _wbpfastclick)
  (set `self.State` 1))

(event `self.OnUpdateMinigame`
  (set `self.CurrentNumberClicks` (+ (`self.CurrentNumberClicks`) 1))
  (`/Game/Game/ui/WBP_FastClick.SetProgress` (`self.WBPFastClick`) (/ (`KismetMathLibrary.Conv_IntToDouble` (`self.CurrentNumberClicks`)) (`KismetMathLibrary.Conv_IntToDouble` (`self.MaxNumberClicks`))))
  (if (>= (`self.CurrentNumberClicks`) (`self.MaxNumberClicks`))
    (`/Game/Game/ui/WBP_FastClick.SetProgress` (`self.WBPFastClick`) 1.0)
    (set `self.State` 2)))

(event `self.OnCompleteMinigame`
  (bind _returnvalue (`self.GiveRecipeToPlayer`))
  (if _returnvalue
    (bind (_direction _scale) (`Timeline|ScaleMesh`)
      (:`Update`
        (`SceneComponent.SetRelativeScale3D` (`self.Mesh`) (`KismetMathLibrary.MakeVector` _scale _scale _scale))
        (`self.UnlockPlayer`)
        (`SceneComponent.SetVisibility` (`self.Widget`) false false :!label _label))
      (:`Finished`
        (set `self.State` 3)))
    (else
      (`self.UnlockPlayer`)
      (goto _label))))

(event `self.Trigger.OnComponentBeginOverlap`
  (params (OverlappedComponent :type "PrimitiveComponent Object Reference") (OtherActor :type "Actor Object Reference") (OtherComp :type "PrimitiveComponent Object Reference") (OtherBodyIndex :type Integer) (bFromSweep :type Boolean) (SweepResult :type "HitResult Structure (by ref)"))
  ;[1 0.4649 0.09567] Trigger Interaction
  (bind _ascoffee_shop_sim_character (cast `CoffeeShopSimCharacter` OtherActor))
  (set `self.PlayerCharacter` _ascoffee_shop_sim_character)
  (`CoffeeShopSimCharacter.OnEnterInteractive` _ascoffee_shop_sim_character self (`self.InteractiveName`))
  (`self.OnPlayerEnterInteractive`))

(event `self.Trigger.OnComponentEndOverlap`
  (params (OverlappedComponent :type "PrimitiveComponent Object Reference") (OtherActor :type "Actor Object Reference") (OtherComp :type "PrimitiveComponent Object Reference") (OtherBodyIndex :type Integer))
  (bind _playercharacter (`self.PlayerCharacter`))
  ;[1 0.4649 0.09567] Trigger Interaction
  (bind _ascoffee_shop_sim_character (cast `CoffeeShopSimCharacter` OtherActor))
  (if (== _ascoffee_shop_sim_character _playercharacter)
    (`CoffeeShopSimCharacter.OnLeaveInteractive` _playercharacter self)
    (set `self.PlayerCharacter` null)
    (`self.OnPlayerLeaveInteractive`)))

(fn `LockPlayer`
  (bind _playercharacter (`self.PlayerCharacter`))
  (bind (_returnvalue_x _returnvalue_y _returnvalue_z) (`KismetMathLibrary.BreakVector` (`self.K2_GetActorLocation` _playercharacter)))
  (bind (_returnvalue_x_2 _returnvalue_y_2) (`KismetMathLibrary.BreakVector` (`SceneComponent.K2_GetComponentLocation` (`self.PlayerPostion`))))
  (`PlayerController.SetCinematicMode` (`GameplayStatics.GetPlayerController` 0) true false false true true)
  (`self.K2_SetActorLocationAndRotation` _playercharacter (`KismetMathLibrary.MakeVector` _returnvalue_x_2 _returnvalue_y_2 _returnvalue_z) (`SceneComponent.K2_GetComponentRotation` (`self.PlayerRotationArrow`)) false false))

(fn `UnlockPlayer`
  (`PlayerController.SetCinematicMode` (`GameplayStatics.GetPlayerController` 0) false false false true true))

(fn `UserConstructionScript`)
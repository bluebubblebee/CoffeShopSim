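; Coffee shop crafting bowl interactive where the player adds held items as recipe ingredients.
; Trigger overlap registers the player; interacting passes the held item to TryAddIngredients, consumes it if accepted and briefly locks input.
; Interacting empty-handed clears the added ingredients.
; Mesh visibility toggles three half-full spheres while the recipe is incomplete, reverting to the empty bowl when ready or cleared; the Full mesh stays hidden.
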(event `self.ReceiveBeginPlay`
  (`parent.ReceiveBeginPlay`)
  (`SceneComponent.SetVisibility` (`self.Full`) false false)
  (`SceneComponent.SetVisibility` (`self.EmptyBowl`) true false)
  (`self.HideBowlHalfFull`))

(event `self.OnInteract`
  (bind _playercharacter (`self.PlayerCharacter`))
  ;[0.7765 0.4549 1] Interact
  (if (not (`self.LockInteractive`))
    (`/Engine/EditorBlueprintResources/StandardMacros.IsValid` _playercharacter
      (:`Is Valid`
        (if (`CoffeeShopSimCharacter.bHasItemOnHands` _playercharacter)
          (bind _returnvalue (`self.TryAddIngredients` (`CoffeeShopSimCharacter.ItemOnHands` _playercharacter)))
          (if _returnvalue
            (set `self.LockInteractive` true)
            (`CoffeeShopSimCharacter.OnGiveItem` (`self.PlayerCharacter`))
            (bind _returnvalue_2 (`self.IsRecipeReady`))
            (if _returnvalue_2
              (`SceneComponent.SetVisibility` (`self.EmptyBowl`) true false)
              (`SceneComponent.SetVisibility` (`self.Full`) false false)
              (`self.HideBowlHalfFull`)
              (else
                (`SceneComponent.SetVisibility` (`self.EmptyBowl`) true false)
                (`SceneComponent.SetVisibility` (`self.Full`) false false)
                (`self.ShowBowlHalfFull`)))
            (`KismetSystemLibrary.Delay` 2.0)
            (set `self.LockInteractive` false))
          (else
            (`KismetArrayLibrary.Array_Clear` (`self.AddedIngredients`))
            (`SceneComponent.SetVisibility` (`self.EmptyBowl`) true false)
            (`SceneComponent.SetVisibility` (`self.Full`) false false)
            (`self.HideBowlHalfFull`)))))))

(event `self.Trigger.OnComponentBeginOverlap`
  (params (OverlappedComponent :type "PrimitiveComponent Object Reference") (OtherActor :type "Actor Object Reference") (OtherComp :type "PrimitiveComponent Object Reference") (OtherBodyIndex :type Integer) (bFromSweep :type Boolean) (SweepResult :type "HitResult Structure (by ref)"))
  ;[0.7765 0.4549 1] Trigger Interaction
  (bind _ascoffee_shop_sim_character (cast `CoffeeShopSimCharacter` OtherActor))
  (set `self.PlayerCharacter` _ascoffee_shop_sim_character)
  (`CoffeeShopSimCharacter.OnEnterInteractive` _ascoffee_shop_sim_character self (`self.InteractiveName`))
  (`self.OnPlayerEnterInteractive`))

(event `self.Trigger.OnComponentEndOverlap`
  (params (OverlappedComponent :type "PrimitiveComponent Object Reference") (OtherActor :type "Actor Object Reference") (OtherComp :type "PrimitiveComponent Object Reference") (OtherBodyIndex :type Integer))
  (bind _playercharacter (`self.PlayerCharacter`))
  ;[0.7765 0.4549 1] Trigger Interaction
  (bind _ascoffee_shop_sim_character (cast `CoffeeShopSimCharacter` OtherActor))
  (if (== _ascoffee_shop_sim_character _playercharacter)
    (`CoffeeShopSimCharacter.OnLeaveInteractive` _playercharacter)
    (set `self.PlayerCharacter` null)
    (`self.OnPlayerLeaveInteractive`)))

(fn `HideBowlHalfFull`
  (`SceneComponent.SetVisibility` (`self.Sphere`) false false)
  (`SceneComponent.SetVisibility` (`self.Sphere1`) false false)
  (`SceneComponent.SetVisibility` (`self.Sphere2`) false false))

(fn `ShowBowlHalfFull`
  (`SceneComponent.SetVisibility` (`self.Sphere`) true false)
  (`SceneComponent.SetVisibility` (`self.Sphere1`) true false)
  (`SceneComponent.SetVisibility` (`self.Sphere2`) true false))

(fn `UserConstructionScript`
  (`parent.UserConstructionScript`))
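; Player controller for the Sim game that routes Enhanced Input actions to handler functions defined outside this Blueprint.
; The in-game graph forwards move, interact and main menu actions, with interact sharing the bottom face button handler.
; The menu graph maps face buttons and menu keys to button and direction handlers.
; IA_LeftButton also drives the LEFT direction, and the menu graph's IA_MainMenu event is unwired.
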(event `EnhancedInput|/Game/Game/Input/InGameActions/IA_Move`
  (params (ActionValue :type "Vector2D Structure") (ElapsedSeconds :type "Float (double-precision)") (TriggeredSeconds :type "Float (double-precision)") (InputAction :type "InputAction Object Reference" :default "/Game/Game/Input/InGameActions/IA_Move.IA_Move"))
  (:`Triggered`
    (`self.HandleMovement` ActionValue)))

(event `EnhancedInput|/Game/Game/Input/InGameActions/IA_Interact`
  (params (ActionValue :type Boolean) (ElapsedSeconds :type "Float (double-precision)") (TriggeredSeconds :type "Float (double-precision)") (InputAction :type "InputAction Object Reference" :default "/Game/Game/Input/InGameActions/IA_Interact.IA_Interact"))
  (:`Started`
    (`self.HandleFaceBottomButton`)))

(event `EnhancedInput|/Game/Game/Input/InGameActions/IA_MainMenu`
  (params (ActionValue :type Boolean) (ElapsedSeconds :type "Float (double-precision)") (TriggeredSeconds :type "Float (double-precision)") (InputAction :type "InputAction Object Reference" :default "/Game/Game/Input/InGameActions/IA_MainMenu.IA_MainMenu"))
  (:`Started`
    (`self.HandleMainMenuButtonInGame`)))

(event `EnhancedInput|/Game/Game/Input/InGameActions/IA_MainMenu`
  (params (ActionValue :type Boolean) (ElapsedSeconds :type "Float (double-precision)") (TriggeredSeconds :type "Float (double-precision)") (InputAction :type "InputAction Object Reference" :default "/Game/Game/Input/InGameActions/IA_MainMenu.IA_MainMenu")))

(event `EnhancedInput|/Game/Game/Input/MenuActions/IA_TopButton`
  (params (ActionValue :type Boolean) (ElapsedSeconds :type "Float (double-precision)") (TriggeredSeconds :type "Float (double-precision)") (InputAction :type "InputAction Object Reference" :default "/Game/Game/Input/MenuActions/IA_TopButton.IA_TopButton"))
  (:`Started`
    (`self.HandleFaceTopButton`)))

(event `EnhancedInput|/Game/Game/Input/MenuActions/IA_RightButton`
  (params (ActionValue :type Boolean) (ElapsedSeconds :type "Float (double-precision)") (TriggeredSeconds :type "Float (double-precision)") (InputAction :type "InputAction Object Reference" :default "/Game/Game/Input/MenuActions/IA_RightButton.IA_RightButton"))
  (:`Started`
    (`self.HandleFaceRightButton`)))

(event `EnhancedInput|/Game/Game/Input/MenuActions/IA_BottomButton`
  (params (ActionValue :type Boolean) (ElapsedSeconds :type "Float (double-precision)") (TriggeredSeconds :type "Float (double-precision)") (InputAction :type "InputAction Object Reference" :default "/Game/Game/Input/MenuActions/IA_BottomButton.IA_BottomButton"))
  (:`Started`
    (`self.HandleFaceBottomButton`)))

(event `EnhancedInput|/Game/Game/Input/MenuActions/IA_LeftButton`
  (params (ActionValue :type Boolean) (ElapsedSeconds :type "Float (double-precision)") (TriggeredSeconds :type "Float (double-precision)") (InputAction :type "InputAction Object Reference" :default "/Game/Game/Input/MenuActions/IA_LeftButton.IA_LeftButton"))
  (:`Started`
    (`self.HandleFaceLeftButton`)))

(event `EnhancedInput|/Game/Game/Input/MenuActions/IA_MenuKeyUp`
  (params (ActionValue :type Boolean) (ElapsedSeconds :type "Float (double-precision)") (TriggeredSeconds :type "Float (double-precision)") (InputAction :type "InputAction Object Reference" :default "/Game/Game/Input/MenuActions/IA_MenuKeyUp.IA_MenuKeyUp"))
  (:`Started`
    (`self.HandleInputDirection` "VE_UP")))

(event `EnhancedInput|/Game/Game/Input/MenuActions/IA_MenuKeyRight`
  (params (ActionValue :type Boolean) (ElapsedSeconds :type "Float (double-precision)") (TriggeredSeconds :type "Float (double-precision)") (InputAction :type "InputAction Object Reference" :default "/Game/Game/Input/MenuActions/IA_MenuKeyRight.IA_MenuKeyRight"))
  (:`Started`
    (`self.HandleInputDirection` "VE_RIGHT")))

(event `EnhancedInput|/Game/Game/Input/MenuActions/IA_MenuKeyDown`
  (params (ActionValue :type Boolean) (ElapsedSeconds :type "Float (double-precision)") (TriggeredSeconds :type "Float (double-precision)") (InputAction :type "InputAction Object Reference" :default "/Game/Game/Input/MenuActions/IA_MenuKeyDown.IA_MenuKeyDown"))
  (:`Started`
    (`self.HandleInputDirection` "VE_DOWN")))

(event `EnhancedInput|/Game/Game/Input/MenuActions/IA_LeftButton`
  (params (ActionValue :type Boolean) (ElapsedSeconds :type "Float (double-precision)") (TriggeredSeconds :type "Float (double-precision)") (InputAction :type "InputAction Object Reference" :default "/Game/Game/Input/MenuActions/IA_LeftButton.IA_LeftButton"))
  (:`Started`
    (`self.HandleInputDirection` "VE_LEFT")))

(fn `UserConstructionScript`)